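; BP_Enemy is a zombie enemy that takes damage and collapses when its health runs out.
; The construction script gives it a random skeletal mesh from the ListZombies list for visual variety.
; Each TakeDamage call subtracts a fixed amount of Health.
; At zero or below, the mesh switches to physics simulation and the capsule's collision is disabled, with no destroy step.
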(event Custom|TakeDamage
  (Variables|Default|SetHealth (- (Variables|Default|GetHealth) 25))
  (if (<= (Variables|Default|GetHealth) 0)
    (Physics|SetSimulatePhysics (Variables|Character|GetMesh) true)
    (Collision|SetCollisionEnabled (Variables|Collision|GetCapsuleComponent) "NoCollision")))

(event EventBeginPlay)

(event Collision|EventActorBeginOverlap
  (params (OtherActor :type Actor%20Object%20Reference)))

(fn ConstructionScript
  (Components|SkeletalMesh|SetSkeletalMeshAsset (Variables|Character|GetMesh) (.OutItem (Utilities|Array|Random (Variables|Default|GetListZombies)))))